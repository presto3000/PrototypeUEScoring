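; BP_LevelActor is a level actor that carries a health bar shown through its HPWidget component.
; On BeginPlay it casts the widget to WB_HealthBar, passes itself as the bar's BPLevelActor reference and hides it.
; ShowHealthBar and HideHealthBar events toggle the bar's visibility, leaving it to other code to decide when it appears.
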(event EventBeginPlay
  (bind _aswb_health_bar (Utilities|Casting|CastToWB_HealthBar (UserInterface|GetUserWidgetObject (Variables|Default|GetHPWidget))))
  (Utilities|IsValid _aswb_health_bar
    (:Is%20Valid
      (Variables|/Game/BLUPRINTS/UI/WB_HealthBar.WB_HealthBar_C|SetBP_LevelActor _aswb_health_bar self)
      (Widget|SetVisibility _aswb_health_bar "Hidden"))))

(event Collision|EventActorBeginOverlap
  (params (OtherActor :type Actor%20Object%20Reference)))

(event EventTick
  (params (DeltaSeconds :type Float%20%28single-precision%29)))

(event EventHideHealthBar
  (bind _aswb_health_bar (Utilities|Casting|CastToWB_HealthBar (UserInterface|GetUserWidgetObject (Variables|Default|GetHPWidget))))
  (Utilities|IsValid _aswb_health_bar
    (:Is%20Valid
      (Widget|SetVisibility _aswb_health_bar "Hidden"))))

(event EventShowHealthBar
  (bind _aswb_health_bar (Utilities|Casting|CastToWB_HealthBar (UserInterface|GetUserWidgetObject (Variables|Default|GetHPWidget))))
  (Utilities|IsValid _aswb_health_bar
    (:Is%20Valid
      (Widget|SetVisibility _aswb_health_bar "Visible"))))

(fn ConstructionScript)